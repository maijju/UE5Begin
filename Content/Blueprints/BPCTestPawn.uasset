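; Test pawn that sets up a Sun, Earth and Moon rotation rig through movement components.
; On BeginPlay, SunRotMove, EarthRotMove and MoonRotMove are bound to the SunRotation, Earth and EarthRotation components respectively.
; Tick and overlap events are empty, and a Move-to-SetActorLocation chain is left unconnected, so it never runs.
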(event EventBeginPlay
  (Components|Movement|SetUpdatedComponent (Variables|Default|GetSunRotMove) (Variables|Default|GetSunRotation))
  (Components|Movement|SetUpdatedComponent (Variables|Default|GetEarthRotMove) (Variables|Default|GetEarth))
  (Components|Movement|SetUpdatedComponent (Variables|Default|GetMoonRotMove) (Variables|Default|GetEarthRotation)))

(event Collision|EventActorBeginOverlap
  (params (OtherActor :type Actor%20Object%20Reference)))

(event EventTick
  (params (DeltaSeconds :type Float%20%28single-precision%29)))

(fn ConstructionScript)